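; Paint volume that paints red vertex color onto BP_TestActor actors inside its sphere at runtime.
; Sphere overlap events maintain the actor list, which Tick processes through a 0.1-second Delay.
; New or moved actors, detected via cached positions, trigger a zero-length, debug-drawn sphere trace at the volume's center.
; The hit location and sphere radius feed PaintVerticesAtLocationV2 on each actor's RuntimeVertexPainting component.
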(event OnComponentBeginOverlap(Sphere)
  (params (OverlappedComponent :type Primitive%20Component%20Object%20Reference) (OtherActor :type Actor%20Object%20Reference) (OtherComp :type Primitive%20Component%20Object%20Reference) (OtherBodyIndex :type Integer) (bFromSweep :type Boolean) (SweepResult :type Hit%20Result%20Structure%20%28by%20ref%29))
  (bind _asbp_test_actor (Utilities|Casting|CastToBP_TestActor OtherActor))
  (Utilities|Array|AddUnique (Variables|Default|GetOverlappingActors) _asbp_test_actor))

(event OnComponentEndOverlap(Sphere)
  (params (OverlappedComponent :type Primitive%20Component%20Object%20Reference) (OtherActor :type Actor%20Object%20Reference) (OtherComp :type Primitive%20Component%20Object%20Reference) (OtherBodyIndex :type Integer))
  (bind _overlappingactors (Variables|Default|GetOverlappingActors))
  (bind _asbp_test_actor (Utilities|Casting|CastToBP_TestActor OtherActor))
  (Utilities|Array|RemoveIndex _overlappingactors (Utilities|Array|FindItem _overlappingactors _asbp_test_actor)))

(event Collision|EventActorBeginOverlap
  (params (OtherActor :type Actor%20Object%20Reference)))

(event EventTick
  (params (DeltaSeconds :type Float%20%28single-precision%29))
  (bind _sphere (Variables|Default|GetSphere))
  (bind (_origin _boxextent _sphereradius) (Collision|GetComponentBounds _sphere))
  (Utilities|FlowControl|Delay 0.1)
  (for _array_element (Variables|Default|GetOverlappingActors)
    (Variables|Default|SetCurrentObject _array_element)
    (if (.ReturnValue (Utilities|Map|Find (Variables|Default|GetCachedPositions) _array_element))
      (if (Utilities|Operators|NotEqual(!=) (.Value (Utilities|Map|Find (Variables|Default|GetCachedPositions) _array_element)) (Transformation|GetActorLocation _array_element) 1.0)
        (bind _outhit (Collision|SphereTraceByChannel _origin _origin _sphereradius "TraceTypeQuery1" false 0 "ForDuration" true "(R=1.000000,G=0.000000,B=0.000000,A=1.000000)" "(R=0.000000,G=1.000000,B=0.000000,A=1.000000)" 2.0 :!label _label))
        (Class|VertexPaintFuncLibrary|PaintVerticesatLocationV2 (Variables|/Game/VertexPainting/Actors/BP_TestActor.BP_TestActor_C|GetRuntimeVertexPainting (Variables|Default|GetCurrentObject)) (.Location (Collision|BreakHitResult _outhit)) (Variables|/Script/Engine.SphereComponent|GetSphereRadius (Variables|Default|GetSphere)) (Math|Color|MakeColor 0 0 255))
        (Utilities|Map|Add (Variables|Default|GetCachedPositions) (Variables|Default|GetCurrentObject) (Transformation|GetActorLocation (Variables|Default|GetCurrentObject))))
      (else
        (goto _label)))))

(fn ConstructionScript)